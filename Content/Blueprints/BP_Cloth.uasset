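; BP_Cloth is a cloth actor Blueprint that exposes reset and drop events and displays the current wind vector.
; ResetCloth and DropCloth events forward to Reset and ReleaseCloth, whose implementations lie outside this graph.
; Each Tick rotates the Scene component along WindVector and scales the Arrow's length by the vector's magnitude.
; The construction script is empty.
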(event Custom|DropCloth
  (Class|Cloth|ReleaseCloth))

(event Custom|ResetCloth
  (Class|Cloth|Reset))

(event EventTick
  (params (DeltaSeconds :type Float%20%28single-precision%29))
  (Transformation|SetWorldRotation (Variables|Default|GetScene) (Math|Conversions|RotationFromXVector (Variables|Default|GetWindVector)) false false)
  ;[1 1 1] Arrow scale
  (Variables|/Script/Engine.ArrowComponent|SetArrowLength (Variables|Default|GetArrow) (* (Math|Vector|VectorLength (Variables|Default|GetWindVector)) 0.07)))

(fn ConstructionScript)